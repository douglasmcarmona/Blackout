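; BP_Battery is a held, usable battery item that recharges a flashlight held in the player's other hand.
; CanBeUsed fetches the opposite-hand item from the attach-parent player and allows use only if that item implements FlashlightInterface, caching it as OtherHandItem.
; Use then sends its BatteryCharge to that item through an interface message and destroys the battery.
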(event `UsageInterface.Use`
  (message `FlashlightInterface.AddBatteryPercentage` (`self.OtherHandItem`) (`self.BatteryCharge`))
  (`self.K2_DestroyActor`))

(fn `CanBeUsed`
  (params (bIsRightHand :type Boolean))
  (returns (ReturnValue :type Boolean))
  (locals (Player :type "Actor Object Reference"))
  (set `local.Player` (`self.GetAttachParentActor`))
  (if (`local.bIsRightHand`)
    (bind _returnvalue (message `HandInterface.GetLeftHandItem` (`local.Player`)))
    (set `self.OtherHandItem` _returnvalue)
    (else
      (bind _returnvalue_2 (message `HandInterface.GetRightHandItem` (`local.Player`)))
      (set `self.OtherHandItem` _returnvalue_2)))
  (return (`KismetSystemLibrary.DoesImplementInterface` (`self.OtherHandItem`) "/Script/Blackout.FlashlightInterface")))

(fn `UserConstructionScript`
  (`parent.UserConstructionScript`))