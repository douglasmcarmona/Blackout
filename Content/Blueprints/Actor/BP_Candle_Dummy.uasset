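; BP_Candle_Dummy is a stand-in candle that lets the player return the held owner candle to the dummy's position.
; On interact, it finds the player through the owner's attach parent and checks which hand holds the owner.
; That hand drops the candle, which runs HandleDrop, takes the dummy's transform, and the dummy destroys itself.
; Construction sets an IsDummyActor flag on a dynamic material and disables flame auto-activation.
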(event `InteractionInterface.Interact`
  (`InteractionInterface.Unhighlight`)
  (bind _output_get (set `self.Player` (`self.GetAttachParentActor` (`self.GetOwner`))))
  (bind _returnvalue (message `HandInterface.GetRightHandItem` _output_get))
  (if (== _returnvalue (`self.GetOwner`))
    (`self.ReturnOwnerCandle` true)
    (else
      (bind _returnvalue_2 (message `HandInterface.GetLeftHandItem` (`self.Player`)))
      (if (== _returnvalue_2 (`self.GetOwner`))
        (`self.ReturnOwnerCandle` false)))))

(fn `ReturnOwnerCandle`
  (params (IsRightHand :type Boolean))
  (locals (Candle :type "Actor Object Reference"))
  (if IsRightHand
    (bind _returnvalue (message `HandInterface.DropRightHandItem` (`self.Player`)))
    (set `local.Candle` _returnvalue)
    (else
      (bind _returnvalue_2 (message `HandInterface.DropLeftHandItem` (`self.Player`)))
      (set `local.Candle` _returnvalue_2)))
  (bind _asbp_interactable_actor (cast `/Game/Blueprints/Actor/BP_InteractableActor` (`local.Candle`)))
  (`self.HandleDrop` _asbp_interactable_actor)
  (`self.K2_SetActorTransform` (`local.Candle`) (`self.GetTransform`) false false)
  (`self.K2_DestroyActor`))

(fn `UserConstructionScript`
  (bind _returnvalue (`KismetMaterialLibrary.CreateDynamicMaterialInstance` "/Game/Assets/Meshes/Candle/M_Candle.M_Candle"))
  (bind _output_get (set `self.CandleDynMat` _returnvalue))
  (`PrimitiveComponent.SetMaterial` (`self.Mesh`) 0 _output_get)
  (`MaterialInstanceDynamic.SetScalarParameterValue` (`self.CandleDynMat`) "IsDummyActor" 1.0)
  (`ActorComponent.SetAutoActivate` (`self.FlameEffect`) false))