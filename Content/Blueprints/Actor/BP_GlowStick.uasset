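; Hand-held glow stick item whose point light burns out over a set lifespan once activated.
; Use requires an empty other hand and makes the stick non-storable; sticks that begin non-storable light up on spawn.
; A looping frame-delta timer scales intensity by a power curve table over normalized lit time.
; Once depleted, it destroys itself after a short delay if not attached to an actor.
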(event `self.ReceiveBeginPlay`
  (`KismetSystemLibrary.DelayUntilNextTick`)
  (if (not (`self.bIsStorable`))
    (`self.StartUsage`)))

(event `UsageInterface.Use`
  (if (`self.bIsStorable`)
    (`self.PlaySoundEffect`)
    (set `self.bIsStorable` false)
    (`self.StartUsage`)))

(event `StartUsage`
  (`SceneComponent.SetVisibility` (`self.PointLight`) true false)
  (`KismetSystemLibrary.K2_SetTimerDelegate` (delegate `Deplete`) (`GameplayStatics.GetWorldDeltaSeconds`) true))

(event `Deplete`
  (bind _returnvalue (`KismetMathLibrary.SafeDivide` (`self.TimeSinceLit`) (`self.PowerLifeSpan`)))
  (bind _outxy (`DataTableFunctionLibrary.EvaluateCurveTableRow` "/Game/Blueprints/Data/CT_GlowStickPower.CT_GlowStickPower" "Power" _returnvalue)
    (:`RowFound`
      (`LightComponent.SetIntensity` (`self.PointLight`) (* _outxy (`self.MaxIntensity`)))
      (if (< _returnvalue 1.0)
        (set `self.TimeSinceLit` (+ (`self.TimeSinceLit`) (`GameplayStatics.GetWorldDeltaSeconds`)))
        (elif (not (`KismetSystemLibrary.IsValid` (`self.GetAttachParentActor`)))
          (`KismetSystemLibrary.Delay` 5.0)
          (`self.K2_DestroyActor`))))))

(fn `CanBeUsed`
  (params (bIsRightHand :type Boolean))
  (returns (ReturnValue :type Boolean))
  (locals (Player :type "Actor Object Reference") (OtherHandItem :type "Actor Object Reference"))
  (set `local.Player` (`self.GetAttachParentActor`))
  (if (`local.bIsRightHand`)
    (bind _returnvalue (message `HandInterface.GetLeftHandItem` (`local.Player`)))
    (set `local.OtherHandItem` _returnvalue)
    (else
      (bind _returnvalue_2 (message `HandInterface.GetRightHandItem` (`local.Player`)))
      (set `local.OtherHandItem` _returnvalue_2)))
  (return (not (`KismetSystemLibrary.IsValid` (`local.OtherHandItem`)))))

(fn `UserConstructionScript`
  (`parent.UserConstructionScript`)
  (`LightComponent.SetIntensity` (`self.PointLight`) (`self.MaxIntensity`))
  (`LocalLightComponent.SetAttenuationRadius` (`self.PointLight`) (`self.AttenuationRadius`))
  (`LightComponent.SetLightColor` (`self.PointLight`) (`self.LightColor`) true)
  (`SceneComponent.SetVisibility` (`self.PointLight`) false false)
  (`LightComponent.SetIndirectLightingIntensity` (`self.PointLight`) 0.0))