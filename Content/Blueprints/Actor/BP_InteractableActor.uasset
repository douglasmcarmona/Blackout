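; BP_InteractableActor is an interactable actor that can show and hide an on-screen interaction prompt.
; ShowInteractWidget creates a WBP_InteractInput for player 0, adds it to the viewport and sets its InteractionText; HideInteractWidget removes it if valid.
; The construction script assigns the mesh a custom depth stencil value but leaves custom depth rendering off.
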(event `self.ShowInteractWidget`
  (bind _returnvalue (`|CreateWidget` "/Game/Blueprints/UI/Gameplay/WBP_InteractInput.WBP_InteractInput_C" (`GameplayStatics.GetPlayerController` 0)))
  (bind _output_get (set `self.InteractWidget` _returnvalue))
  (`UserWidget.AddToViewport` _output_get 0)
  (`/Game/Blueprints/UI/Gameplay/WBP_InteractInput.SetInteractText` (`self.InteractWidget`) (`self.InteractionText`)))

(event `self.HideInteractWidget`
  (bind _interactwidget (`self.InteractWidget`)
    (:`then`
      (`Widget.RemoveFromParent` _interactwidget))
    (:`else`)))

(fn `UserConstructionScript`
  (`PrimitiveComponent.SetCustomDepthStencilValue` (`self.Mesh`) 250)
  (`PrimitiveComponent.SetRenderCustomDepth` (`self.Mesh`) false))