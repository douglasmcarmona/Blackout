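; BP_InteractableSpawner is a placed actor that spawns one random interactable at its location when play begins.
; It picks a class at random from InteractableActorOptions and, if valid, spawns it using the spawner's rotation, adjusting for collisions but always spawning.
; Glow sticks (BP_GlowStick) are a special case and get an extra quarter turn of yaw.
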(event `self.ReceiveBeginPlay`
  (bind _returnvalue (`self.K2_GetActorRotation`))
  (bind _output_get (set `self.InteractableClass` (`KismetArrayLibrary.Array_Random` (`self.InteractableActorOptions`))))
  (if (`KismetSystemLibrary.IsValidClass` _output_get)
    (`|SpawnActorFromClass` (`self.InteractableClass`) (`KismetMathLibrary.MakeTransform` (`self.K2_GetActorLocation`) (select `bool` (== (`self.InteractableClass`) "/Game/Blueprints/Actor/BP_GlowStick.BP_GlowStick_C") :`false` _returnvalue :`true` (`KismetMathLibrary.MakeRotator` (.roll _returnvalue) (.pitch _returnvalue) (+ (.yaw _returnvalue) 90.0)))) "AdjustIfPossibleButAlwaysSpawn" "MultiplyWithRoot" null null)))

(fn `UserConstructionScript`)