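; Interactable one-shot lever that flips when used and signals its activation.
; The Flick timeline swings the lever mesh's pitch through a half turn from its starting angle, with a separate Start event playing it at reduced speed.
; When the swing finishes, it disables collision on both meshes, spawns sparks that respect the SFX setting and calls Activated.
; Construction disables physics and makes the lever mesh the highlight target.
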(event `self.ReceiveBeginPlay`
  (`SceneComponent.K2_SetRelativeRotation` (`self.LeverMesh`) (struct :`Pitch` 15.0) false false)
  (set `self.LeverInitialRotation` (`SceneComponent.RelativeRotation` (`self.LeverMesh`))))

(event `InteractionInterface.Interact`
  (bind (_returnvalue_location _returnvalue_rotation) (`KismetMathLibrary.BreakTransform` (`self.GetTransform`)))
  (bind (_leverinitialrotation_roll _leverinitialrotation_pitch) (`KismetMathLibrary.BreakRotator` (`self.LeverInitialRotation`)))
  (bind (_direction _leverpitchalpha) (`Timeline|Flick` :!via `PlayFromStart`)
    (:`Update`
      (`SceneComponent.K2_SetRelativeRotation` (`self.LeverMesh`) (`KismetMathLibrary.MakeRotator` 0.0 (+ _leverinitialrotation_pitch (`KismetMathLibrary.Lerp` 0.0 -180.0 _leverpitchalpha))) false false))
    (:`Finished`
      (`PrimitiveComponent.SetCollisionEnabled` (`self.LeverMesh`) "NoCollision")
      (`PrimitiveComponent.SetCollisionEnabled` (`self.Mesh`) "NoCollision")
      (bind _returnvalue (`NiagaraFunctionLibrary.SpawnSystemAtLocation` (`self.SparksEffect`) (- _returnvalue_location (0.0 0.0 30.0)) _returnvalue_rotation))
      (`NiagaraComponent.SetVariableBool` _returnvalue "IsSFXEnabled" (`BlackoutFunctionLibrary.IsSFXEnabled` null))
      (`self.Activated`))))

(event `Start`
  (`TimelineComponent.SetPlayRate` (`self.Flick`) 0.25)
  (`TimelineComponent.Play` (`self.Flick`)))

(fn `UserConstructionScript`
  (`parent.UserConstructionScript`)
  (`PrimitiveComponent.SetSimulatePhysics` (`self.Mesh`) false)
  (`PrimitiveComponent.SetSimulatePhysics` (`self.LeverMesh`) false)
  (`self.SetHighlightTarget` (`self.LeverMesh`)))