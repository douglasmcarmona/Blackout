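; BP_PaperNote is a hand-held, throwable note item that displays text looked up by its note ID.
; Use toggles a reading widget, blocks storage while open and updates the character's reading state; CanBeUsed prevents reading both hands' notes at once.
; The ID persists through inventory slot data.
; Thrown or initially non-storable notes self-destroy after a delay, and a burn timeline drives a dissolve on the dynamic material.
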(event `self.ReceiveBeginPlay`
  (`self.SetPaperNoteText`)
  (`KismetSystemLibrary.DelayUntilNextTick`)
  (if (not (`self.bIsStorable`))
    (`self.TimedDestroy`)))

(event `UsageInterface.Use`
  (bind _asbp_blackout_character (cast `/Game/Blueprints/Characters/BP_BlackoutCharacter` (`self.GetAttachParentActor`))
    (:`then`
      (set `self.BlackoutCharacter` _asbp_blackout_character))
    (:`CastFailed`
      _))
  (if (`self.IsBeingUsed`)
    (set `self.IsBeingUsed` false)
    (bind _papernotewidget (`self.PaperNoteWidget`)
      (:`then`
        (`Widget.RemoveFromParent` _papernotewidget)
        (set `self.bIsStorable` true)
        (`self.UpdatePlayerReadingStatus`))
      (:`else`))
    (else
      (set `self.IsBeingUsed` true)
      (bind _returnvalue (`|CreateWidget` "/Game/Blueprints/UI/Gameplay/WBP_PaperNoteCanvas.WBP_PaperNoteCanvas_C" (`GameplayStatics.GetPlayerController` 0)))
      (bind _output_get (set `self.PaperNoteWidget` _returnvalue))
      (`UserWidget.AddToViewport` _output_get 0)
      (`/Game/Blueprints/UI/Gameplay/WBP_PaperNote.SetText` (`/Game/Blueprints/UI/Gameplay/WBP_PaperNoteCanvas.WBP_PaperNote` (`self.PaperNoteWidget`)) (`self.Text`))
      (set `self.bIsStorable` false)
      (`self.UpdatePlayerReadingStatus`))))

(event `InteractionInterface.Throw`
  (params (ThrowForce :type "Vector Structure (by ref)"))
  (`parent.Throw` ThrowForce)
  (set `self.bIsStorable` false)
  (`self.TimedDestroy`))

(event `TimedDestroy`
  (`PrimitiveComponent.SetCollisionResponseToChannel` (`self.Mesh`) "ECC_Visibility" "ECR_Ignore")
  (`KismetSystemLibrary.Delay` 5.0)
  (`self.TimerFinished`)
  (`self.K2_DestroyActor`))

(event `BurnEvent`
  (bind (_direction _burnalpha) (`Timeline|Burn` :!via `PlayFromStart`)
    (:`Update`
      (`MaterialInstanceDynamic.SetScalarParameterValue` (`self.PaperDynMat`) "DissolveScale" _burnalpha)
      (`MaterialInstanceDynamic.SetScalarParameterValue` (`self.PaperDynMat`) "DissolveProgress" _burnalpha))))

(fn `CanBeUsed`
  (params (bIsRightHand :type Boolean))
  (returns (ReturnValue :type Boolean))
  (locals (Player :type "Actor Object Reference") (OtherHandItem :type "Actor Object Reference") (RetVal :type Boolean))
  (set `local.Player` (`self.GetAttachParentActor`))
  (if (`local.bIsRightHand`)
    (bind _returnvalue (message `HandInterface.GetLeftHandItem` (`local.Player`)))
    (set `local.OtherHandItem` _returnvalue)
    (else
      (bind _returnvalue_2 (message `HandInterface.GetRightHandItem` (`local.Player`)))
      (set `local.OtherHandItem` _returnvalue_2)))
  (bind _asbp_paper_note (cast `/Game/Blueprints/Actor/BP_PaperNote` (`local.OtherHandItem`))
    (:`then`
      (set `local.RetVal` (not (`/Game/Blueprints/Actor/BP_PaperNote.IsBeingUsed` _asbp_paper_note))))
    (:`CastFailed`
      (set `local.RetVal` true)))
  (return (`local.RetVal`)))

(fn `HandleStoredItemSlotData`
  (params (SlotData :type "SlotData Structure (by ref)"))
  (`BlueprintMapLibrary.Map_Add` (`.IntegerValues` (break `SlotData` SlotData)) (`self.PaperNoteIdMapKey`) (`self.PaperNoteId`))
  (return))

(fn `HandleWithdrawnItemSlotData`
  (params (SlotData :type "SlotData Structure (by ref)"))
  (set `self.PaperNoteId` (`BlueprintMapLibrary.Map_Find` (`.IntegerValues` (break `SlotData` SlotData)) (`self.PaperNoteIdMapKey`)))
  (`self.SetPaperNoteText`)
  (return))

(fn `SetPaperNoteText`
  (set `self.Text` (`.PaperNoteText` (break `PaperNote` (`PaperNoteInfo.FindPaperNoteById` (`BlackoutFunctionLibrary.GetPaperNoteInfo` null) (`self.PaperNoteId`))))))

(fn `UpdatePlayerReadingStatus`
  (bind _blackoutcharacter (`self.BlackoutCharacter`)
    (:`then`
      (set `BlackoutCharacter.bIsReadingNote` (`self.IsBeingUsed`) _blackoutcharacter))
    (:`else`)))

(fn `UserConstructionScript`
  (`parent.UserConstructionScript`)
  (bind _returnvalue (`PrimitiveComponent.CreateDynamicMaterialInstance` (`self.Mesh`) 0 "/Game/Assets/Meshes/Paper_Note/M_PaperNote.M_PaperNote" "None"))
  (bind _output_get (set `self.PaperDynMat` _returnvalue))
  (`PrimitiveComponent.SetMaterial` (`self.Mesh`) 0 _output_get))