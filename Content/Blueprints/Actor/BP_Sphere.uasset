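; BP_Sphere is a usable hand-held item that requires the player to hold a BP_Cone in the other hand.
; CanBeUsed finds the BP_BlackoutCharacter with GetActorOfClass, queries the hand opposite the one given, and returns whether that item is a cone.
; Use is a simple event that only prints an on-screen message with the item's display name, without repeating the check.
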(event `UsageInterface.Use`
  (`KismetSystemLibrary.PrintString` (`KismetStringLibrary.Concat_StrStr` "You have used the item " (`KismetSystemLibrary.GetDisplayName` self)) true true (struct :`R` 1.0 :`G` 0.860204 :`A` 1.0) 10.0))

(fn `CanBeUsed`
  (params (bIsRightHand :type Boolean))
  (returns (ReturnValue :type Boolean))
  (locals (Player :type "/Game/Blueprints/Characters/BP_BlackoutCharacter Object Reference"))
  (bind _returnvalue (`GameplayStatics.GetActorOfClass` "/Game/Blueprints/Characters/BP_BlackoutCharacter.BP_BlackoutCharacter_C"))
  (set `local.Player` _returnvalue)
  (if (`local.bIsRightHand`)
    (bind _returnvalue_2 (message `HandInterface.GetLeftHandItem` (`local.Player`)))
    (return (`GameplayStatics.ObjectIsA` _returnvalue_2 "/Game/Blueprints/Actor/BP_Cone.BP_Cone_C"))
    (else
      (bind _returnvalue_3 (message `HandInterface.GetRightHandItem` (`local.Player`)))
      (return (`GameplayStatics.ObjectIsA` _returnvalue_3 "/Game/Blueprints/Actor/BP_Cone.BP_Cone_C")))))

(fn `UserConstructionScript`
  (`parent.UserConstructionScript`))