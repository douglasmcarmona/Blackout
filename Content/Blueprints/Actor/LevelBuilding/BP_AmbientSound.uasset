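; BP_AmbientSound is a level-placed actor that plays an ambient sound while respecting the game's music setting.
; On BeginPlay it registers a callback with the BlackoutGameInstance music-toggle delegate.
; The callback stops the sound when music is disabled and restarts it when enabled, provided CanPlay is set.
; A Play event starts the sound only if music is enabled.
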(event `self.ReceiveBeginPlay`
  (bind _asblackout_game_instance (cast `BlackoutGameInstance` (`GameplayStatics.GetGameInstance`)))
  (add `BlackoutGameInstance.OnMusicToggledDelegate` _asblackout_game_instance (delegate `OnMusicToggledDelegate_Event`)))

(event `OnMusicToggledDelegate_Event`
  (params (bMusicEnabled :type Boolean))
  (if bMusicEnabled
    (if (`self.CanPlay`)
      (`AudioComponent.Play` (`self.AmbientSound`) 0.0))
    (else
      (`AudioComponent.Stop` (`self.AmbientSound`)))))

(event `Play`
  (if (`BlackoutFunctionLibrary.IsMusicEnabled` null)
    (`AudioComponent.Play` (`self.AmbientSound`) 0.0)))

(fn `UserConstructionScript`)