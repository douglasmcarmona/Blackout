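; BP_DungeonSection_Base is a base actor for dungeon sections used in level building, with a configurable light fixture.
; Its construction script creates a dynamic M_Light material on the LightMesh's second slot and sets its emissive color from LightColor.
; The same color and a LightIntensity value drive the PointLight, keeping fixture glow and cast light matched in color.
; The event graph holds no runtime logic.
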(fn `UserConstructionScript`
  (bind _returnvalue (`PrimitiveComponent.CreateDynamicMaterialInstance` (`self.LightMesh`) 1 "/Game/Assets/Meshes/MazeWallLight/M_Light.M_Light" "None"))
  (bind _output_get (set `self.LightMaterial` _returnvalue))
  (`PrimitiveComponent.SetMaterial` (`self.LightMesh`) 1 _output_get)
  (`MaterialInstanceDynamic.SetVectorParameterValue` (`self.LightMaterial`) "EmissiveColor" (`self.LightColor`))
  (`LightComponent.SetLightColor` (`self.PointLight`) (`self.LightColor`) true)
  (`LightComponent.SetIntensity` (`self.PointLight`) (`self.LightIntensity`)))