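; BP_DungeonSection_Corner is a level-building actor that provides a configurable corner piece for dungeons.
; Its construction script checks Render booleans for the start arch, finish arch, floor and ceiling, destroying each component whose flag is off.
; The event graph holds only disabled placeholder events, so the actor adds no runtime logic of its own.
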(fn `UserConstructionScript`
  (`|ExecutionSequence`
    (:`then_0`
      (if (not (`self.RenderArchStart`))
        (`ActorComponent.K2_DestroyComponent` (`self.ArchStart`))))
    (:`then_1`
      (if (not (`self.RenderArchFinish`))
        (`ActorComponent.K2_DestroyComponent` (`self.ArchFinish`))))
    (:`then_2`
      (if (not (`self.RenderFloor`))
        (`ActorComponent.K2_DestroyComponent` (`self.Floor`))))
    (:`then_3`
      (if (not (`self.RenderCeiling`))
        (`ActorComponent.K2_DestroyComponent` (`self.Ceiling`))))))