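; BP_DungeonSection_Straight is a level-building actor that provides a straight dungeon section with floor, arch and ceiling components.
; Its construction script checks the RenderFloor, RenderArch and RenderCeiling flags and destroys each component whose flag is off, so each instance can omit parts.
; The event graph holds only disabled stub events, so the Blueprint adds no runtime logic.
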(fn `UserConstructionScript`
  (`|ExecutionSequence`
    (:`then_0`
      (if (not (`self.RenderFloor`))
        (`ActorComponent.K2_DestroyComponent` (`self.Floor`))))
    (:`then_1`
      (if (not (`self.RenderArch`))
        (`ActorComponent.K2_DestroyComponent` (`self.Arch`))))
    (:`then_2`
      (if (not (`self.RenderCeiling`))
        (`ActorComponent.K2_DestroyComponent` (`self.Ceiling`))))))