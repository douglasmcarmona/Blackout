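; Level-end trigger actor that runs the victory sequence when BP_BlackoutCharacter overlaps its FinishVolume.
; It shows an end-game widget, disables input, hides the pause button and, if music is enabled, crossfades tag-located ambient sounds from default to win.
; After a short delay it opens the victory menu with a final note including elapsed game time, enables the cursor and destroys both held items.
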(event `self.ReceiveBeginPlay`
  (`|ExecutionSequence`
    (:`then_0`
      (bind _outactors (`GameplayStatics.GetAllActorsWithTag` "DefaultAmbientSound"))
      (bind _asbp_ambient_sound (cast `/Game/Blueprints/Actor/LevelBuilding/BP_AmbientSound` (`|GetArrayItem` _outactors)))
      (bind _output_get (set `self.DefaultAmbientSound` _asbp_ambient_sound))
      (`/Game/Blueprints/Actor/LevelBuilding/BP_AmbientSound.Play` _output_get))
    (:`then_1`
      (bind _outactors_2 (`GameplayStatics.GetAllActorsWithTag` "WinAmbientSound"))
      (bind _asbp_ambient_sound_2 (cast `/Game/Blueprints/Actor/LevelBuilding/BP_AmbientSound` (`|GetArrayItem` _outactors_2)))
      (set `self.WinAmbientSound` _asbp_ambient_sound_2))))

(event `self.FinishVolume.OnComponentBeginOverlap`
  (params (OverlappedComponent :type "PrimitiveComponent Object Reference") (OtherActor :type "Actor Object Reference") (OtherComp :type "PrimitiveComponent Object Reference") (OtherBodyIndex :type Integer) (bFromSweep :type Boolean) (SweepResult :type "HitResult Structure (by ref)"))
  (bind _returnvalue (`GameplayStatics.GetPlayerController` 0))
  (bind _asbp_blackout_character (cast `/Game/Blueprints/Characters/BP_BlackoutCharacter` OtherActor))
  (set `self.Player` _asbp_blackout_character)
  (`|ExecutionSequence`
    (:`then_0`
      (`self.ShowEndGameWidget`)
      (`self.ChangeAmbientSound`)
      (`BlackoutFunctionLibrary.TogglePauseButton` null)
      (`self.DisableInput` (`Controller.K2_GetPawn` _returnvalue) _returnvalue))
    (:`then_1`
      (`KismetSystemLibrary.Delay` 3.0)
      (bind _endgamewidget (`self.EndGameWidget`)
        (:`then`
          (`Widget.RemoveFromParent` _endgamewidget)
          (`self.ShowVictoryMenu`)
          (`WidgetBlueprintLibrary.SetInputMode_UIOnlyEx` (`GameplayStatics.GetPlayerController` 0) null)
          (set `PlayerController.bShowMouseCursor` true (`GameplayStatics.GetPlayerController` 0))
          (`self.EmptyHands`))
        (:`else`)))))

(fn `ChangeAmbientSound`
  (locals (FadeDuration :type "Float (double-precision)" :default 1.0))
  (if (`BlackoutFunctionLibrary.IsMusicEnabled` null)
    (`AudioComponent.FadeOut` (`/Game/Blueprints/Actor/LevelBuilding/BP_AmbientSound.AmbientSound` (`self.DefaultAmbientSound`)) (`local.FadeDuration`) 0.0 "Linear")
    (`AudioComponent.FadeIn` (`/Game/Blueprints/Actor/LevelBuilding/BP_AmbientSound.AmbientSound` (`self.WinAmbientSound`)) (`local.FadeDuration`) 1.0 0.0 "Linear")))

(fn `EmptyHands`
  (`|ExecutionSequence`
    (:`then_0`
      (bind _returnvalue (message `HandInterface.GetLeftHandItem` (`self.Player`)))
      (`/Engine/EditorBlueprintResources/StandardMacros.IsValid` _returnvalue
        (:`Is Valid`
          (`self.K2_DestroyActor` _returnvalue))))
    (:`then_1`
      (bind _returnvalue_2 (message `HandInterface.GetRightHandItem` (`self.Player`)))
      (`/Engine/EditorBlueprintResources/StandardMacros.IsValid` _returnvalue_2
        (:`Is Valid`
          (`self.K2_DestroyActor` _returnvalue_2))))))

(fn `GetFinalNoteText`
  (returns (FormattedText :type Text))
  (bind _returnvalue (/ (`KismetSystemLibrary.GetGameTimeInSeconds`) 60.0))
  (bind _returnvalue_2 (`KismetMathLibrary.FTrunc` _returnvalue))
  (return (`|FormatText` "{PaperNoteText} \n \n{TimeText}" (`.PaperNoteText` (break `PaperNote` (`PaperNoteInfo.FindPaperNoteById` (`BlackoutFunctionLibrary.GetPaperNoteInfo` null) 1))) (`|FormatText` "Oh, and by the way, you took {MinutesText}{SecondsText} to get out. Do whatever you want with that information" (`KismetMathLibrary.SelectText` (`|FormatText` "{Minutes} {Minutes}|plural(one=minute, other=minutes) and " _returnvalue_2) "" (> _returnvalue_2 0)) (`|FormatText` "{Seconds} {Seconds}|plural(one=second, other=seconds)" (`KismetMathLibrary.FTrunc` (* (`KismetMathLibrary.Fraction` _returnvalue) 60.0)))))))

(fn `ShowEndGameWidget`
  (bind _returnvalue (`|CreateWidget` "/Game/Blueprints/UI/Gameplay/WBP_EndGame.WBP_EndGame_C" (`GameplayStatics.GetPlayerController` 0)))
  (bind _output_get (set `self.EndGameWidget` _returnvalue))
  (`UserWidget.AddToViewport` _output_get 0))

(fn `ShowVictoryMenu`
  (bind _returnvalue (`|CreateWidget` "/Game/Blueprints/UI/Gameplay/VictoryMenu/WBP_VictoryMenu.WBP_VictoryMenu_C" (`GameplayStatics.GetPlayerController` 0) (`self.GetFinalNoteText`)))
  (bind _output_get (set `self.VictoryWidget` _returnvalue))
  (`UserWidget.AddToViewport` _output_get 0))

(fn `UserConstructionScript`)