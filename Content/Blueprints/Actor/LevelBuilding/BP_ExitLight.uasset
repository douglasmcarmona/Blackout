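; BP_ExitLight is a level light actor that changes to its configured color when a lever is activated.
; On BeginPlay it finds a single BP_Lever with GetActorOfClass and binds to its Activated event, which applies LightColor.
; The construction script creates a dynamic material for the light mesh, starts the light black, sets the point light intensity and shows the ceiling.
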(event `self.ReceiveBeginPlay`
  (bind _returnvalue (`GameplayStatics.GetActorOfClass` "/Game/Blueprints/Actor/BP_Lever.BP_Lever_C"))
  (add `/Game/Blueprints/Actor/BP_Lever.Activated` _returnvalue (delegate `CustomEvent`)))

(event `CustomEvent`
  (`self.SetPointLightColor` (`self.LightColor`)))

(fn `UserConstructionScript`
  (bind _returnvalue (`PrimitiveComponent.CreateDynamicMaterialInstance` (`self.LightMesh`) 1 "/Game/Assets/Meshes/MazeLight/M_Light.M_Light" "None"))
  (bind _output_get (set `self.LightMaterial` _returnvalue))
  (`PrimitiveComponent.SetMaterial` (`self.LightMesh`) 1 _output_get)
  ; Suggested default color: BC8003FF
  (`self.SetPointLightColor` (struct))
  (`LightComponent.SetIntensity` (`self.PointLight`) (`self.LightIntensity`))
  (`SceneComponent.SetVisibility` (`self.Ceiling`) true false))