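; BP_MazeLight is a maze light fixture that goes dark when a lever is activated.
; Its Construction Script creates a dynamic material for the light mesh, applies the configured color and intensity, and shows the ceiling mesh.
; A shared function keeps emissive and point light color in sync.
; On BeginPlay it binds to the first BP_Lever found in the level, whose Activated event sets that color to black.
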(event `self.ReceiveBeginPlay`
  (bind _returnvalue (`GameplayStatics.GetActorOfClass` "/Game/Blueprints/Actor/BP_Lever.BP_Lever_C"))
  (add `/Game/Blueprints/Actor/BP_Lever.Activated` _returnvalue (delegate `Activated_Event`)))

(event `Activated_Event`
  (`self.SetPointLightColor` (struct)))

(fn `SetPointLightColor`
  (params (Color :type "LinearColor Structure"))
  (`MaterialInstanceDynamic.SetVectorParameterValue` (`self.LightMaterial`) "EmissiveColor" Color)
  (`LightComponent.SetLightColor` (`self.PointLight`) Color true))

(fn `UserConstructionScript`
  (bind _returnvalue (`PrimitiveComponent.CreateDynamicMaterialInstance` (`self.LightMesh`) 1 "/Game/Assets/Meshes/MazeLight/M_Light.M_Light" "None"))
  (bind _output_get (set `self.LightMaterial` _returnvalue))
  (`PrimitiveComponent.SetMaterial` (`self.LightMesh`) 1 _output_get)
  ; Suggested default color: BC8003FF
  (`self.SetPointLightColor` (`self.LightColor`))
  (`LightComponent.SetIntensity` (`self.PointLight`) (`self.LightIntensity`))
  (`SceneComponent.SetVisibility` (`self.Ceiling`) true false))