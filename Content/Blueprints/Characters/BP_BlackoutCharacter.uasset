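; Player character Blueprint for Blackout that handles charged throwing of items held in either hand, plus pause toggling.
; EnableThrow input shows a charge-bar widget bound to the character while active.
; ThrowItem's axis sign picks the hand; holding builds clamped charge, triggering throws along control rotation, and canceling drops with zero force.
; Item interface messages check throwability and apply the throw after detaching, with throwing blocked while reading notes.
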(event `EnhancedInput|/Game/Input/IA_EnableThrow`
  (params (ActionValue :type Boolean) (ElapsedSeconds :type "Float (double-precision)") (TriggeredSeconds :type "Float (double-precision)") (InputAction :type "InputAction Object Reference" :default "/Game/Input/IA_EnableThrow.IA_EnableThrow"))
  (:`Started`
    (bind _returnvalue (`|CreateWidget` "/Game/Blueprints/UI/Gameplay/WBP_ThrowObjectCharge.WBP_ThrowObjectCharge_C" (`GameplayStatics.GetPlayerController` 0) (`self.UseGradientChargeBar`)))
    (bind _output_get (set `self.ThrowChargeUI` _returnvalue))
    (`UserWidget.AddToViewport` _output_get 0)
    (`/Game/Blueprints/UI/Gameplay/WBP_ThrowObjectCharge.SetWidgetController` (`self.ThrowChargeUI`) self)
    (set `/Game/Blueprints/UI/Gameplay/WBP_ThrowObjectCharge.UseGradient` (`self.UseGradientChargeBar`) (`self.ThrowChargeUI`)))
  (:`Completed`
    (`Widget.RemoveFromParent` (`self.ThrowChargeUI`))))

(event `EnhancedInput|/Game/Input/IA_ThrowItem`
  (params (ActionValue :type "Float (double-precision)") (ElapsedSeconds :type "Float (double-precision)") (TriggeredSeconds :type "Float (double-precision)") (InputAction :type "InputAction Object Reference" :default "/Game/Input/IA_ThrowItem.IA_ThrowItem"))
  (:`Triggered`
    (if (`self.CanThrowItem`)
      (`self.ThrowObject` (`self.GetThrowForce`))
      (`KismetSystemLibrary.Delay` 0.5)
      (set `self.bHasJustThrownItem` false)))
  (:`Started`
    (set `self.IsRightHand` (> ActionValue 0.0)))
  (:`Ongoing`
    (if (`self.CanThrowItem`)
      (bind _output_get (set `self.ChargeTime` (`KismetMathLibrary.FClamp` ElapsedSeconds 0.0 (`self.MaxChargeTime`))))
      (`self.ThrowCharge` (/ _output_get (`self.MaxChargeTime`)) (`self.IsRightHand`))))
  (:`Canceled`
    (if (`self.CanThrowItem`)
      (`self.ThrowObject` (`KismetMathLibrary.Vector_Zero`))
      (`KismetSystemLibrary.Delay` 0.5)
      (set `self.bHasJustThrownItem` false))))

(event `EnhancedInput|/Game/Input/IA_PauseMenu`
  (params (ActionValue :type Boolean) (ElapsedSeconds :type "Float (double-precision)") (TriggeredSeconds :type "Float (double-precision)") (InputAction :type "InputAction Object Reference" :default "/Game/Input/IA_PauseMenu.IA_PauseMenu"))
  (:`Triggered`
    (set `MovementComponent.Velocity` (0.0 0.0 0.0) (`self.CharacterMovement`))
    (`BlackoutFunctionLibrary.ToggleGamePaused` null (not (`GameplayStatics.IsGamePaused`)))))

(fn `CanThrowItem`
  (returns (CanThrow :type Boolean))
  (locals (IsItemThrowable :type Boolean))
  (if (`self.IsRightHand`)
    (bind _righthanditem (`self.RightHandItem`)
      (:`then`
        (bind _returnvalue (message `InteractionInterface.IsThrowable` _righthanditem))
        (set `local.IsItemThrowable` _returnvalue))
      (:`else`
        (set `local.IsItemThrowable` false)))
    (else
      (bind _lefthanditem (`self.LeftHandItem`)
        (:`then`
          (bind _returnvalue_2 (message `InteractionInterface.IsThrowable` _lefthanditem))
          (set `local.IsItemThrowable` _returnvalue_2))
        (:`else`
          (set `local.IsItemThrowable` false)))))
  (return (and (`self.bIsThrowEnabled`) (`local.IsItemThrowable`) (not (`self.bIsReadingNote`)))))

(fn `GetThrowForce`
  (returns (ReturnValue :type "Vector Structure"))
  (return (* (`KismetMathLibrary.Conv_RotatorToVector` (`self.GetControlRotation`)) (* (/ (`self.ChargeTime`) (`self.MaxChargeTime`)) (`self.MaxThrowForceMagnitude`)))))

(fn `IsFlashlight`
  (params (InteractableActor :type "Actor Object Reference"))
  (returns (ReturnValue :type Boolean))
  (return (`GameplayStatics.ObjectIsA` InteractableActor)))

(fn `ThrowObject`
  (params (ThrowForce :type "Vector Structure"))
  (if (`self.IsRightHand`)
    (bind _righthanditem (`self.RightHandItem`)
      (:`then`
        (`self.K2_DetachFromActor` _righthanditem "KeepWorld" "KeepWorld" "KeepWorld")
        (message `InteractionInterface.Throw` (`self.RightHandItem`) (`local.ThrowForce`))
        (set `self.RightHandItem` null))
      (:`else`))
    (else
      (bind _lefthanditem (`self.LeftHandItem`)
        (:`then`
          (`self.K2_DetachFromActor` _lefthanditem "KeepWorld" "KeepWorld" "KeepWorld")
          (message `InteractionInterface.Throw` (`self.LeftHandItem`) (`local.ThrowForce`))
          (set `self.LeftHandItem` null))
        (:`else`))))
  (`self.ThrowCharge` 0.0 (`self.IsRightHand`))
  (set `self.bHasJustThrownItem` true))

(fn `UserConstructionScript`)