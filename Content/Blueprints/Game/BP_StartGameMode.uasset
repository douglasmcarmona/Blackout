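; BP_StartGameMode runs the game's opening flow, from seizure warning to start menu.
; On BeginPlay it disables pawn input, shows WBP_SeizureWarning after a short delay, then fades it out.
; When the fade finishes, it plays the level's LevelSequenceActor, whose completion creates WBP_GameStart and shows its buttons.
; Each stage is chained by finish delegates, and the menu's fade-in end switches to UI-only input with a visible cursor.
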(event `self.ReceiveBeginPlay`
  (`|ExecutionSequence`
    (:`then_0`
      (`self.DisableInput` (`GameplayStatics.GetPlayerPawn` 0) (`GameplayStatics.GetPlayerController` 0)))
    (:`then_1`
      (`KismetSystemLibrary.Delay` 2.0)
      (bind _returnvalue (`|CreateWidget` "/Game/Blueprints/UI/Gameplay/GameStartMenu/WBP_SeizureWarning.WBP_SeizureWarning_C"))
      (bind _output_get (set `self.WarningWidget` _returnvalue))
      (`UserWidget.AddToViewport` _output_get 0)
      (add `/Game/Blueprints/UI/Gameplay/GameStartMenu/WBP_SeizureWarning.FadeOutFinished` (`self.WarningWidget`) (delegate `FadeOutFinished_Event`))
      (`KismetSystemLibrary.Delay` 7.5)
      (`/Game/Blueprints/UI/Gameplay/GameStartMenu/WBP_SeizureWarning.FadeOut` (`self.WarningWidget`)))))

(event `FadeOutFinished_Event`
  (`Widget.RemoveFromParent` (`self.WarningWidget`))
  (bind _returnvalue (`GameplayStatics.GetActorOfClass` "/Script/LevelSequence.LevelSequenceActor"))
  (bind _sequenceplayer (`LevelSequenceActor.SequencePlayer` _returnvalue)
    (:`then`
      (add `MovieSceneSequencePlayer.OnFinished` _sequenceplayer (delegate `OnFinished_Event`))
      (`KismetSystemLibrary.Delay` 1.0)
      (`MovieSceneSequencePlayer.Play` _sequenceplayer))
    (:`else`)))

(event `OnFinished_Event`
  (bind _returnvalue (`|CreateWidget` "/Game/Blueprints/UI/Gameplay/GameStartMenu/WBP_GameStart.WBP_GameStart_C" (`GameplayStatics.GetPlayerController` 0)))
  (bind _output_get (set `self.GameStartWidget` _returnvalue))
  (add `/Game/Blueprints/UI/Gameplay/GameStartMenu/WBP_GameStart.FadeInFinished` _output_get (delegate `FadeInFinished_Event`))
  (`UserWidget.AddToViewport` (`self.GameStartWidget`) 0)
  (`/Game/Blueprints/UI/Gameplay/GameStartMenu/WBP_GameStart.ShowButtons` (`self.GameStartWidget`)))

(event `FadeInFinished_Event`
  (`WidgetBlueprintLibrary.SetInputMode_UIOnlyEx` (`GameplayStatics.GetPlayerController` 0) null)
  (set `PlayerController.bShowMouseCursor` true (`GameplayStatics.GetPlayerController` 0)))

(fn `UserConstructionScript`)